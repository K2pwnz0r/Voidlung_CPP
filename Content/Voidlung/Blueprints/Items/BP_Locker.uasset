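; BP_Locker is an interactable locker with an animated door, apparently a hiding spot built on a parent class.
; Interact locks out further use, swings the door open with a timeline, then calls the parent Interact once it finishes.
; The HidingED event, bound on BeginPlay, plays a closing timeline that re-enables interaction when done.
; Both timelines call PlaySound2D on every update.
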(event `self.ReceiveBeginPlay`
  (`parent.ReceiveBeginPlay`)
  (add `self.HidingED` (delegate `HidingED_Event`)))

(event `HidingED_Event`
  (`self.CloseDoor`))

(event `/Game/Voidlung/Blueprints/Systems/BPI_Interactable.Interact`
  (if (`self.CanInteract`)
    (set `self.CanInteract` false)
    (bind (_direction _alpha) (`Timeline|OpenDoor` :!via `PlayFromStart`)
      (:`Update`
        (`SceneComponent.K2_SetRelativeRotation` (`self.LockerDoor`) (`KismetMathLibrary.MakeRotator` 0.0 0.0 (`KismetMathLibrary.Lerp` 0.0 100.0 _alpha)) false false)
        ;[1 1 1] Add Open Door Sound Here
        (`GameplayStatics.PlaySound2D` null 1.0 1.0 0.0 null null))
      (:`Finished`
        (`parent.Interact`)))))

(event `CloseDoor`
  (bind (_direction _alpha) (`Timeline|CloseLockerDoor` :!via `PlayFromStart`)
    (:`Update`
      (`SceneComponent.K2_SetRelativeRotation` (`self.LockerDoor`) (`KismetMathLibrary.MakeRotator` 0.0 0.0 (`KismetMathLibrary.Lerp` 100.0 0.0 _alpha)) false false)
      ;[1 1 1] Add Close Door Sound Here
      (`GameplayStatics.PlaySound2D` null 1.0 1.0 0.0 null null))
    (:`Finished`
      (set `self.CanInteract` true))))

(fn `UserConstructionScript`
  (`parent.UserConstructionScript`))