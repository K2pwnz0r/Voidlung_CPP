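; BP_Generator is an objective generator that the player stabilizes through a voltage calibration minigame.
; Once StartCalibration resets and activates it, Tick constantly decays the voltage and raises it while InputHeld is true.
; Keeping input held with voltage inside the target zone accumulates hold time until CompleteStabilization ends calibration and plays a sound.
; InteractionBox overlap handlers track PlayerInRange, but nothing here reads that flag or sets InputHeld.
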(event `PlayerOutOfRange`
  (params (OverlappedComponent :type "PrimitiveComponent Object Reference") (OtherActor :type "Actor Object Reference") (OtherComp :type "PrimitiveComponent Object Reference") (OtherBodyIndex :type Integer))
  (add `PrimitiveComponent.OnComponentEndOverlap` (`self.InteractionBox`) (delegate `PlayerOutOfRange`))
  (cast `/Game/FirstPerson/Blueprints/BP_FirstPersonCharacter` (`GameplayStatics.GetPlayerCharacter` 0))
  (set `self.bPlayerInRange` false))

(event `PlayerInRange`
  (params (OverlappedComponent :type "PrimitiveComponent Object Reference") (OtherActor :type "Actor Object Reference") (OtherComp :type "PrimitiveComponent Object Reference") (OtherBodyIndex :type Integer) (bFromSweep :type Boolean) (SweepResult :type "HitResult Structure (by ref)"))
  (add `PrimitiveComponent.OnComponentBeginOverlap` (`self.InteractionBox`) (delegate `PlayerInRange`))
  (cast `/Game/FirstPerson/Blueprints/BP_FirstPersonCharacter` (`GameplayStatics.GetPlayerCharacter` 0))
  (set `self.bPlayerInRange` true))

(event `self.ReceiveBeginPlay`
  (`self.EnableInput` (`GameplayStatics.GetPlayerController` 0)))

(event `self.ReceiveTick`
  (params (DeltaSeconds :type "Float (single-precision)"))
  ;[1 1 1] Updates Interaction
  (if (and (== (`self.bIsCalibrating`) true) (== (`self.bIsStabilized`) false))
    (set `self.VoltageValue` (- (`self.VoltageValue`) (* (`self.VoltageDecayRate`) DeltaSeconds)))
    (if (== (`self.bInputHeld`) true)
      (set `self.VoltageValue` (+ (`self.VoltageValue`) (* (`self.VoltageSpeed`) DeltaSeconds)))
      (set `self.VoltageValue` (`KismetMathLibrary.FClamp` (`self.VoltageValue`)))
      (if (and (>= (`self.VoltageValue`) (`self.TargetZoneMin`)) (<= (`self.VoltageValue`) (`self.TargetZoneMax`)))
        (set `self.CurrentHoldTime` (+ (`self.CurrentHoldTime`) DeltaSeconds))
        (if (>= (`self.CurrentHoldTime`) (`self.StabilizeTime`))
          (`self.CompleteStabilization`))
        (else
          (set `self.CurrentHoldTime` 0.0))))))

(event `CompleteStabilization`
  (set `self.bIsStabilized` true)
  (set `self.bIsCalibrating` false)
  (`GameplayStatics.PlaySound2D` null 1.0 1.0 0.0 null null))

(event `StartCalibration`
  (set `self.bIsCalibrating` true)
  (set `self.CurrentHoldTime` 0.0)
  (set `self.VoltageValue` 0.0))

(fn `UserConstructionScript`)